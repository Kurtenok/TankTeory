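; Game mode Blueprint for Toon Tanks that puts up the start and end-of-game screens.
; The StartGame event creates the start widget and adds it to the viewport.
; The GameOver event creates the end widget and sets its display text to a win or lose message based on the WonGame flag.
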(event `self.StartGame`
  (bind _returnvalue (`|CreateWidget` "/Game/BluePrints/Widgets/WBP_StartGameWidget.WBP_StartGameWidget_C"))
  (`UserWidget.AddToViewport` _returnvalue 0))

(event `self.GameOver`
  (params (bWonGame :type Boolean))
  (bind _returnvalue (`|CreateWidget` "/Game/BluePrints/Widgets/WBP_EndGameWidget.WBP_EndGameWidget_C"))
  (`UserWidget.AddToViewport` _returnvalue 0)
  (if bWonGame
    (set `self.GameOverMessage` "You Won!")
    (else
      (set `self.GameOverMessage` "You Lose!")))
  (`TextBlock.SetText` (`/Game/BluePrints/Widgets/WBP_EndGameWidget.DisplayText` _returnvalue) (`KismetTextLibrary.Conv_StringToText` (`self.GameOverMessage`))))

(fn `UserConstructionScript`)